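; Door Blueprint that slides open vertically for the Player and can start locked behind a key.
; Entering the Trigger while locked spends one of the Player's Keys to unlock it for good, then plays the Open timeline.
; The timeline drives the Door's relative Z, playing from start on entry and reversing from end on exit whenever unlocked.
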(event `self.Trigger.OnComponentBeginOverlap`
  (params (OverlappedComponent :type "PrimitiveComponent Object Reference") (OtherActor :type "Actor Object Reference") (OtherComp :type "PrimitiveComponent Object Reference") (OtherBodyIndex :type Integer) (bFromSweep :type Boolean) (SweepResult :type "HitResult Structure (by ref)"))
  (bind _asplayer (cast `/Game/Blueprints/Player/Player` OtherActor))
  (if (`self.Locked`)
    (bind _keys (`/Game/Blueprints/Player/Player.Keys` _asplayer))
    (if (> _keys 0)
      (`/Engine/EditorBlueprintResources/StandardMacros.DecrementInt` _keys
        (:`  `
          (set `self.Locked` false)
          (bind (_direction _newtrack_0) (`Timeline|Open` :!via `PlayFromStart` :!label _label)
            (:`Update`
              (`SceneComponent.K2_SetRelativeLocation` (`self.Door`) (* (0.0 0.0 1.0) _newtrack_0) false false))))))
    (else
      (goto _label :!via `PlayFromStart`))))

(event `self.Trigger.OnComponentEndOverlap`
  (params (OverlappedComponent :type "PrimitiveComponent Object Reference") (OtherActor :type "Actor Object Reference") (OtherComp :type "PrimitiveComponent Object Reference") (OtherBodyIndex :type Integer))
  (cast `/Game/Blueprints/Player/Player` OtherActor)
  (if (not (`self.Locked`))
    (goto _label :!via `ReverseFromEnd`)))

(fn `UserConstructionScript`)