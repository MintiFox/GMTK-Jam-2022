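; Bouncer is an enemy character that chases the player while its room is loaded and hurts them on contact.
; Tick moves and turns it toward the player reference passed in on room load.
; A bad die result from DiceCapture rescales its walk speed by the rolled value.
; Overlap deals damage with knockback and plays a bounce montage, while hits taken launch it and destroy it once health drops below zero.
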(event `self.ReceiveBeginPlay`
  (set `self.CurrentHealth` (`self.MaxHealth`))
  (bind _returnvalue (`GameplayStatics.GetActorOfClass` "/Game/Blueprints/HUD/DiceCapture.DiceCapture_C"))
  (add `/Game/Blueprints/HUD/DiceCapture.OnBadDieResult` _returnvalue (delegate `OnBadDie`)))

(event `OnBadDie`
  (params (DieResult :type Integer))
  (set `CharacterMovementComponent.MaxWalkSpeed` (`KismetMathLibrary.Conv_IntToDouble` (* DieResult 200)) (`self.CharacterMovement`)))

(event `self.ReceiveTick`
  (params (DeltaSeconds :type "Float (single-precision)"))
  (bind _returnvalue (`KismetMathLibrary.Normal` (- (`self.K2_GetActorLocation` (`self.Player Ref`)) (`self.K2_GetActorLocation`))))
  (set `self.Delta Seconds` DeltaSeconds)
  (if (`self.Loaded`)
    (`self.AddMovementInput` _returnvalue)
    (`self.K2_SetActorRotation` (`KismetMathLibrary.MakeRotFromX` _returnvalue))))

(event `/Game/Blueprints/Interface/Enemy.OnRoomLoad`
  (params (PlayerRef :type "/Game/Blueprints/Player/Player Object Reference"))
  (set `self.Player Ref` PlayerRef)
  (set `self.Loaded` true))

(event `/Game/Blueprints/Interface/Enemy.OnRoomUnload`
  (set `self.Loaded` false))

(event `/Game/Blueprints/Interface/CanDamage.OnDamaged`
  (params (Damage :type Integer) (Knockback :type "Vector Structure"))
  (`self.LaunchCharacter` Knockback true true)
  (set `self.CurrentHealth` (- (`self.CurrentHealth`) Damage))
  (if (< (`self.CurrentHealth`) 0)
    (`self.K2_DestroyActor`)))

(event `self.ReceiveActorBeginOverlap`
  (params (OtherActor :type "Actor Object Reference"))
  (bind _asplayer (cast `/Game/Blueprints/Player/Player` OtherActor))
  (`/Game/Blueprints/Player/Player.OnDamaged` _asplayer 1 (* (`KismetMathLibrary.Normal` (- (`self.K2_GetActorLocation` (`self.Player Ref`)) (`self.K2_GetActorLocation`))) (`self.Knockback`)))
  (`|PlayMontage` (`self.Mesh`) "/Game/Characters/Bouncer/Anim/AnimM_Bounce.AnimM_Bounce" 1.3))

(fn `UserConstructionScript`)