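; Roulette sawblade hazard that travels back and forth along a spline and damages actors it touches, with its speed driven by bad dice rolls.
; A looping PingPong timeline moves RouletteWheel along the spline.
; DiceCapture's bad-die event sets Speed from the result, scaling both timeline play rate and per-tick blade spin, which ignores delta time.
; Overlaps send a damage message without knockback only while Speed exceeds a small threshold.
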(event `self.ReceiveBeginPlay`
  (bind _returnvalue (`GameplayStatics.GetActorOfClass` "/Game/Blueprints/HUD/DiceCapture.DiceCapture_C"))
  (add `/Game/Blueprints/HUD/DiceCapture.OnBadDieResult` _returnvalue (delegate `OnBadDie`))
  (`TimelineComponent.SetLooping` (`self.PingPong`) true)
  (bind (_direction _newtrack_0) (`Timeline|PingPong` :!via `PlayFromStart`)
    (:`Update`
      (`SceneComponent.K2_SetWorldLocation` (`self.RouletteWheel`) (`SplineComponent.GetLocationAtTime` (`self.Spline`) _newtrack_0 "World" false) false true))))

(event `OnBadDie`
  (params (DieResult :type Integer))
  (bind _output_get (set `self.Speed` (* DieResult 0.1)))
  (`TimelineComponent.SetPlayRate` (`self.PingPong`) _output_get))

(event `/Game/Blueprints/Interface/Enemy.OnRoomLoad`
  (params (PlayerRef :type "/Game/Blueprints/Player/Player Object Reference"))
  (set `self.Player Ref` PlayerRef))

(event `self.ReceiveTick`
  (params (DeltaSeconds :type "Float (single-precision)"))
  (bind _roulettesawblade (`self.RouletteSawblade`))
  (bind (_relativerotation_roll _relativerotation_pitch _relativerotation_yaw) (`KismetMathLibrary.BreakRotator` (`SceneComponent.RelativeRotation` _roulettesawblade)))
  (set `self.Delta Seconds` DeltaSeconds)
  (`SceneComponent.K2_SetRelativeRotation` _roulettesawblade (`KismetMathLibrary.MakeRotator` 0.0 0.0 (+ _relativerotation_yaw (* (`self.Speed`) 5.0))) false false))

(event `self.RouletteWheel.OnComponentBeginOverlap`
  (params (OverlappedComponent :type "PrimitiveComponent Object Reference") (OtherActor :type "Actor Object Reference") (OtherComp :type "PrimitiveComponent Object Reference") (OtherBodyIndex :type Integer) (bFromSweep :type Boolean) (SweepResult :type "HitResult Structure (by ref)"))
  (if (> (`self.Speed`) 0.1)
    (message `/Game/Blueprints/Interface/CanDamage.OnDamaged` OtherActor (`self.Damage`) (0.0 0.0 0.0))))

(fn `UserConstructionScript`)