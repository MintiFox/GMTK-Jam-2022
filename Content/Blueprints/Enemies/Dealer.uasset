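; Dealer is an enemy that shoots DealerBullet projectiles at the player while its room is loaded.
; Room load stores the player reference and starts a looping fire-rate timer, which room unload clears.
; Each shot spawns at the Dealer's transform, with its direction set toward the player's location at that moment.
; Damage reduces health, which starts at maximum, and the actor is destroyed only when health drops below zero.
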(event `self.ReceiveBeginPlay`
  (set `self.CurrentHealth` (`self.MaxHealth`)))

(event `self.ReceiveTick`
  (params (DeltaSeconds :type "Float (single-precision)")))

(event `/Game/Blueprints/Interface/Enemy.OnRoomLoad`
  (params (PlayerRef :type "/Game/Blueprints/Player/Player Object Reference"))
  (set `self.Player Ref` PlayerRef)
  (`KismetSystemLibrary.PrintString` "LoadedEnemy")
  (bind _returnvalue (`KismetSystemLibrary.K2_SetTimerDelegate` (delegate `Fire`) (`self.FireRate`) true))
  (set `self.EnemyFire` _returnvalue))

(event `Fire`
  (bind _returnvalue (`|SpawnActorFromClass` "/Game/Blueprints/Bullets/DealerBullet.DealerBullet_C" (`self.GetTransform`) "Undefined" "OverrideRootScale" null null))
  (set `/Game/Blueprints/Bullets/BulletBase.Direction` (`KismetMathLibrary.Normal` (- (`self.K2_GetActorLocation` (`self.Player Ref`)) (`self.K2_GetActorLocation`))) _returnvalue))

(event `/Game/Blueprints/Interface/Enemy.OnRoomUnload`
  (`KismetSystemLibrary.K2_ClearAndInvalidateTimerHandle` (`self.EnemyFire`)))

(event `/Game/Blueprints/Interface/CanDamage.OnDamaged`
  (params (Damage :type Integer) (Knockback :type "Vector Structure"))
  (`KismetSystemLibrary.PrintString` "HIT")
  (set `self.CurrentHealth` (- (`self.CurrentHealth`) Damage))
  (if (< (`self.CurrentHealth`) 0)
    (`self.K2_DestroyActor`)))

(fn `UserConstructionScript`)