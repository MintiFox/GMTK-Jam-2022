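; Room camera actor that takes over the view and activates the room's enemies when the player enters its overlap area.
; On overlap by the tagged player, it cubic-blends the first player controller's view target to itself.
; It then sends a room-load message with the player reference to valid ObjectsToEnable entries implementing the Enemy interface.
; When the player leaves, those enemies receive an unload message, while the view target stays unchanged.
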(event `self.ReceiveBeginPlay`)

(event `self.ReceiveActorBeginOverlap`
  (params (OtherActor :type "Actor Object Reference"))
  (if (`self.ActorHasTag` OtherActor "Player")
    (`self.EnableCam`)
    (bind _asplayer (cast `/Game/Blueprints/Player/Player` OtherActor))
    (set `self.PlayerRef` _asplayer)
    (for _array_element (`self.ObjectsToEnable`)
      (if (`KismetSystemLibrary.IsValid` _array_element)
        (if (`KismetSystemLibrary.DoesImplementInterface` _array_element "/Game/Blueprints/Interface/Enemy.Enemy_C")
          (message `/Game/Blueprints/Interface/Enemy.OnRoomLoad` _array_element (`self.PlayerRef`)))))))

(event `self.ReceiveActorEndOverlap`
  (params (OtherActor :type "Actor Object Reference"))
  (bind _asplayer (cast `/Game/Blueprints/Player/Player` OtherActor))
  (set `self.PlayerRef` _asplayer)
  (for _array_element (`self.ObjectsToEnable`)
    (if (`KismetSystemLibrary.IsValid` _array_element)
      (if (`KismetSystemLibrary.DoesImplementInterface` _array_element "/Game/Blueprints/Interface/Enemy.Enemy_C")
        (message `/Game/Blueprints/Interface/Enemy.OnRoomUnload` _array_element)))))

(event `EnableCam`
  (`PlayerController.SetViewTargetWithBlend` (`GameplayStatics.GetPlayerController` 0) self 1.0 "VTBlend_Cubic" 0.0 true))

(fn `UserConstructionScript`)