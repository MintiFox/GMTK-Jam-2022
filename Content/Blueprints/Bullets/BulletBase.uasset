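; BulletBase is a base projectile Blueprint that flies in a straight line and damages the opposing side.
; Tick moves it by Direction and Speed with a swept offset, and BeginPlay destroys it after its Lifespan.
; On overlap, PlayerAligned selects the Enemy or Player tag to match.
; Valid targets implementing CanDamage receive Damage and directional Knockback through OnDamagedMessage, then the bullet destroys itself after a brief delay.
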(event `self.ReceiveTick`
  (params (DeltaSeconds :type "Float (single-precision)"))
  ;[1 1 1] MoveBullet
  (`self.K2_AddActorWorldOffset` (* (* (`self.Direction`) (`self.Speed`)) DeltaSeconds) true))

(event `self.ReceiveBeginPlay`
  ;[1 1 1] Kill at end of lifespan
  (`KismetSystemLibrary.Delay` (`self.Lifespan`))
  (`self.K2_DestroyActor`))

(event `self.ReceiveActorBeginOverlap`
  (params (OtherActor :type "Actor Object Reference"))
  ;[1 1 1] OnOverlap
  (if (`self.ActorHasTag` OtherActor (select `bool` (`self.PlayerAligned`) :`false` "Player" :`true` "Enemy" :!type "Name"))
    (if (`KismetSystemLibrary.DoesImplementInterface` OtherActor "/Game/Blueprints/Interface/CanDamage.CanDamage_C")
      (message `/Game/Blueprints/Interface/CanDamage.OnDamaged` OtherActor (`self.Damage`) (* (`self.Direction`) (`self.Knockback`)))
      (`KismetSystemLibrary.Delay` 0.05)
      (`self.K2_DestroyActor`))))

(fn `UserConstructionScript`)