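; Bomb projectile that is launched along its direction and explodes after a set lifespan rather than on contact.
; On begin play it pushes its physics sphere, then after the delay spawns explosion effects and runs a sphere overlap sized by actor scale.
; Hit actors implementing CanDamage receive damage and outward knockback, while other hits that are BombableWalls are destroyed, and the bomb then destroys itself.
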(event `self.ReceiveBeginPlay`
  (`KismetSystemLibrary.Delay` 0.01)
  (`PrimitiveComponent.AddForce` (`self.Sphere`) (* (`self.Direction`) (`self.Speed`)) "None" true)
  (`KismetSystemLibrary.Delay` (`self.Lifespan`))
  (`GameplayStatics.SpawnEmitterAtLocation` "/Game/StarterContent/Particles/P_Explosion.P_Explosion" (`self.K2_GetActorLocation`) (struct) (`self.GetActorRelativeScale3D`))
  (`GameplayStatics.PlaySoundAtLocation` "/Game/StarterContent/Audio/Explosion_Cue.Explosion_Cue" (`self.K2_GetActorLocation`) (struct) 1.0 1.0 0.0 null null null)
  (bind _outactors (`KismetSystemLibrary.SphereOverlapActors` (`self.K2_GetActorLocation`) (* (`KismetMathLibrary.VSize` (`self.GetActorRelativeScale3D`)) 200.0) (`self.Object Types`)))
  (for _array_element _outactors
    (`KismetSystemLibrary.PrintString` (`KismetSystemLibrary.GetDisplayName` _array_element))
    (if (`KismetSystemLibrary.DoesImplementInterface` _array_element "/Game/Blueprints/Interface/CanDamage.CanDamage_C")
      (message `/Game/Blueprints/Interface/CanDamage.OnDamaged` _array_element (`self.Damage`) (* (`KismetMathLibrary.Normal` (- (`self.K2_GetActorLocation` _array_element) (`self.K2_GetActorLocation`))) (`self.Knockback`)))
      (else
        (bind _asbombable_wall (cast `/Game/SuperGrid/StarterPack/Materials/Palette/Grids/BombableWall` _array_element))
        (`self.K2_DestroyActor` _asbombable_wall))))
  (`KismetSystemLibrary.Delay` 0.01)
  (`self.K2_DestroyActor`))

(event `self.ReceiveActorBeginOverlap`
  (params (OtherActor :type "Actor Object Reference")))

(event `self.ReceiveTick`
  (params (DeltaSeconds :type "Float (single-precision)"))
  (set `self.Delta Seconds` DeltaSeconds))

(fn `UserConstructionScript`
  (`parent.UserConstructionScript`))