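; DiceCapture actor that continuously rolls a good die and a bad die, each shown as a cube.
; On BeginPlay both loops start, each using a timeline to tumble its cube with random rotations.
; When a timeline finishes, the cube snaps to one of six preset face rotations and the random index is broadcast through that die's result dispatcher.
; Each die re-rolls after a fixed delay; only the good die plays sounds.
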(event `self.ReceiveBeginPlay`
  (`self.GenerateGoodDieNumbers`)
  (`self.GenerateBadDieNumbers`))

(event `GenerateGoodDieNumbers`
  (`GameplayStatics.PlaySound2D` "/Game/Audio/SFX/DiceWoosh/Spiin.Spiin" 1.0 1.0 0.0 null null)
  ;[1 1 1] GenerateNewNumbers
  (bind (_direction _newtrack_0) (`Timeline|Spin` :!via `PlayFromStart`)
    (:`Update`
      (`SceneComponent.K2_AddWorldRotation` (`self.Cube`) (`KismetMathLibrary.Conv_VectorToRotator` (* (`KismetMathLibrary.RandomUnitVector`) _newtrack_0)) false false))
    (:`Finished`
      (set `self.RandomSelection` (`KismetMathLibrary.RandomIntegerInRange` 0 5))
      (`SceneComponent.K2_SetWorldRotation` (`self.Cube`) (select `int` (`self.RandomSelection`) :`0` (`self.1`) :`1` (`self.2`) :`2` (`self.3`) :`3` (`self.4`) :`4` (`self.5`) :`5` (`self.6`)) false false)
      (`GameplayStatics.PlaySound2D` null 1.0 1.0 0.0 null null)
      (`self.OnGoodDieResult` (`self.RandomSelection`))
      (`KismetSystemLibrary.Delay` 10.0)
      (`self.GenerateGoodDieNumbers`))))

(event `GenerateBadDieNumbers`
  ;[1 1 1] GenerateNewNumbers
  (bind (_direction _newtrack_0) (`Timeline|Timeline_0` :!via `PlayFromStart`)
    (:`Update`
      (`SceneComponent.K2_AddWorldRotation` (`self.Cube1`) (`KismetMathLibrary.Conv_VectorToRotator` (* (`KismetMathLibrary.RandomUnitVector`) _newtrack_0)) false false))
    (:`Finished`
      (set `self.RandomSelection` (`KismetMathLibrary.RandomIntegerInRange` 0 5))
      (`SceneComponent.K2_SetWorldRotation` (`self.Cube1`) (select `int` (`self.RandomSelection`) :`0` (`self.1`) :`1` (`self.2`) :`2` (`self.3`) :`3` (`self.4`) :`4` (`self.5`) :`5` (`self.6`)) false false)
      (`self.OnBadDieResult` (`self.RandomSelection`))
      (`KismetSystemLibrary.Delay` 10.0)
      (`self.GenerateBadDieNumbers`))))

(fn `UserConstructionScript`)