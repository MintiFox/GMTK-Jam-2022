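; Slot machine chest that dispenses a random spawnable when the player overlaps its cube, once only unless InfiniteUse is set.
; After a short delay it plays a sound, spawns an item from Spawnables and moves it above the machine.
; Weapon pickups get a random WeaponDrops weapon and use LaunchFromMachine; other items are thrown by force on their static mesh.
; An item with neither loops back to the cast with no exit.
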(event `self.Cube.OnComponentBeginOverlap`
  (params (OverlappedComponent :type "PrimitiveComponent Object Reference") (OtherActor :type "Actor Object Reference") (OtherComp :type "PrimitiveComponent Object Reference") (OtherBodyIndex :type Integer) (bFromSweep :type Boolean) (SweepResult :type "HitResult Structure (by ref)"))
  (bind (_returnvalue_location _returnvalue_rotation) (`KismetMathLibrary.BreakTransform` (`self.GetTransform`)))
  (bind _returnvalue (+ (* (`self.GetActorRightVector`) 5000.0) (* (`self.GetActorUpVector`) 45000.0)))
  (if (not (`self.Used`))
    (cast `/Game/Blueprints/Player/Player` OtherActor)
    (`KismetSystemLibrary.Delay` 0.5)
    (`GameplayStatics.PlaySoundAtLocation` "/Game/Audio/SFX/SlotMachine/SlotMachine.SlotMachine" (`self.K2_GetActorLocation`) (struct) 1.0 1.0 0.0 null null null)
    (bind _returnvalue_2 (`|SpawnActorFromClass` (`KismetArrayLibrary.Array_Random` (`self.Spawnables`)) (`KismetMathLibrary.MakeTransform` _returnvalue_location _returnvalue_rotation) "Undefined" "OverrideRootScale" null null))
    (if (not (`self.InfiniteUse`))
      (set `self.Used` true))
    (`self.K2_SetActorLocation` _returnvalue_2 (+ (+ (* (`self.GetActorRightVector`) 10.0) (* (`self.GetActorUpVector`) 275.0)) (`self.K2_GetActorLocation`)) false false)
    (bind _asweapon_pickup (cast `/Game/Blueprints/Weapons/WeaponPickup` _returnvalue_2 :!label _label)
      (:`then`
        (set `/Game/Blueprints/Weapons/WeaponPickup.Weapon` (`KismetArrayLibrary.Array_Random` (`self.WeaponDrops`)) _asweapon_pickup)
        (`KismetSystemLibrary.Delay` 0.025)
        (`/Game/Blueprints/Weapons/WeaponPickup.LaunchFromMachine` _asweapon_pickup _returnvalue))
      (:`CastFailed`
        (bind _returnvalue_3 (`self.GetComponentByClass` _returnvalue_2 "/Script/Engine.StaticMeshComponent"))
        (if (`KismetSystemLibrary.IsValid` _returnvalue_3)
          (`PrimitiveComponent.AddForce` _returnvalue_3 _returnvalue "None" true)
          (else
            (goto _label)))))))

(fn `UserConstructionScript`)