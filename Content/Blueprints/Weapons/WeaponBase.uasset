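; Weapon base Blueprint whose stats are set by a dice roll through its OnGoodRoll function.
; The passed Level selects one of six per-level values, Level1 through Level6.
; DiceStat decides whether that value overwrites Speed, Damage, Fire Rate or Size, with Damage truncated to an integer.
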(fn `OnGoodRoll`
  (params (Level :type Integer))
  (locals (SelectedStat :type "Float (double-precision)"))
  (set `local.SelectedStat` (select `int` Level :`0` (`self.level 1`) :`1` (`self.level 2`) :`2` (`self.level 3`) :`3` (`self.level 4`) :`4` (`self.level 5`) :`5` (`self.level 6`)))
  (switch `/Game/Blueprints/Weapons/WeaponUpgradeStats` (`self.DiceStat`)
    (:`NewEnumerator0`
      (set `self.Speed` (`local.SelectedStat`)))
    (:`NewEnumerator1`
      (set `self.Damage` (`KismetMathLibrary.FTrunc` (`local.SelectedStat`))))
    (:`NewEnumerator2`
      (set `self.FireRate` (`local.SelectedStat`)))
    (:`NewEnumerator3`
      (set `self.Size` (`local.SelectedStat`)))))