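; Trigger volume that activates a set of enemies when the player enters it.
; On overlap with a Player, it stores the reference and sends OnRoomLoad through the Enemy interface to each valid actor in its ObjectsToEnable array, passing the player along.
; It then disables the box's collision so it fires only once.
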(event `self.ReceiveActorBeginOverlap`
  (params (OtherActor :type "Actor Object Reference"))
  (bind _asplayer (cast `/Game/Blueprints/Player/Player` OtherActor))
  (set `self.PlayerRef` _asplayer)
  (`KismetSystemLibrary.PrintString` "Enemies Activated")
  (for _array_element (`self.ObjectsToEnable`)
    (if (`KismetSystemLibrary.IsValid` _array_element)
      (if (`KismetSystemLibrary.DoesImplementInterface` _array_element "/Game/Blueprints/Interface/Enemy.Enemy_C")
        (message `/Game/Blueprints/Interface/Enemy.OnRoomLoad` _array_element (`self.PlayerRef`)))))
  (`PrimitiveComponent.SetCollisionEnabled` (`self.Box`) "NoCollision"))

(fn `UserConstructionScript`)