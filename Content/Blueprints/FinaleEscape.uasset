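; FinaleEscape is an actor that runs an escape sequence in which a pile rises and damages the player on contact.
; When the Player overlaps StartingTrigger, the trigger disables itself and the view blends to this actor.
; One timeline then drives both the pile's height and the camera's position along a spline, while the camera yaws using delta seconds cached from Tick.
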(event `self.ReceiveTick`
  (params (DeltaSeconds :type "Float (single-precision)"))
  (set `self.Delta Seconds` DeltaSeconds))

(event `Start`
  (bind _risingpile (`self.RisingPile`))
  (bind (_returnvalue_x _returnvalue_y) (`KismetMathLibrary.BreakVector` (`SceneComponent.K2_GetComponentLocation` _risingpile)))
  (`PlayerController.SetViewTargetWithBlend` (`GameplayStatics.GetPlayerController` 0) self 1.0 "VTBlend_Cubic" 0.0 true)
  (bind (_direction _newtrack_0 _camtrack) (`Timeline|Timeline_0` :!via `PlayFromStart`)
    (:`Update`
      (`SceneComponent.K2_SetWorldLocation` _risingpile (`KismetMathLibrary.MakeVector` _returnvalue_x _returnvalue_y _newtrack_0) false false)
      (`SceneComponent.K2_SetWorldLocation` (`self.Camera`) (`SplineComponent.GetLocationAtTime` (`self.CameraSplie`) _camtrack "World" false) false false)
      (`SceneComponent.K2_AddWorldRotation` (`self.Camera`) (`KismetMathLibrary.MakeRotator` 0.0 0.0 (* (`self.CamRotateSpeed`) (`self.Delta Seconds`))) false false))))

(event `self.StartingTrigger.OnComponentBeginOverlap`
  (params (OverlappedComponent :type "PrimitiveComponent Object Reference") (OtherActor :type "Actor Object Reference") (OtherComp :type "PrimitiveComponent Object Reference") (OtherBodyIndex :type Integer) (bFromSweep :type Boolean) (SweepResult :type "HitResult Structure (by ref)"))
  (cast `/Game/Blueprints/Player/Player` OtherActor)
  (`PrimitiveComponent.SetCollisionEnabled` (`self.StartingTrigger`) "NoCollision")
  (`self.Start`))

(event `self.RisingPile.OnComponentBeginOverlap`
  (params (OverlappedComponent :type "PrimitiveComponent Object Reference") (OtherActor :type "Actor Object Reference") (OtherComp :type "PrimitiveComponent Object Reference") (OtherBodyIndex :type Integer) (bFromSweep :type Boolean) (SweepResult :type "HitResult Structure (by ref)"))
  (bind _asplayer (cast `/Game/Blueprints/Player/Player` OtherActor))
  (`/Game/Blueprints/Interface/CanDamage.OnDamaged` _asplayer 100 (0.0 0.0 0.0)))

(fn `UserConstructionScript`)