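; Player character for a shooter with camera-relative movement, independent stick or mouse-trace aim, and dice-levelled weapons.
; Good die results from DiceCapture re-equip the weapon at that level, and ammo-limited pickups revert to the base weapon when empty.
; A looping fire-rate timer spawns spread projectiles using weapon stats.
; Damage applies knockback and brief invincibility, while death ragdolls the mesh and reloads the level.
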(event `self.ReceiveTick`
  (params (DeltaSeconds :type "Float (single-precision)"))
  (bind _camera (`self.Camera`))
  (set `self.Delta Seconds` DeltaSeconds)
  ;[1 1 1] Walking
  (`self.AddMovementInput` (`self.MoveInput`))
  (`self.PlayerRotate`)
  ;[1 1 1] Reset Inputs
  (set `self.AimInput` (0.0 0.0 0.0))
  (set `self.MoveInput` (0.0 0.0 0.0))
  (set `self.RotateCatchup` (`KismetMathLibrary.FInterpTo` (`self.RotateCatchup`) (`self.RotateOffset`) (`GameplayStatics.GetWorldDeltaSeconds`) 10.0))
  (`SceneComponent.K2_SetWorldRotation` (`self.Camera`) (`KismetMathLibrary.RInterpTo` (`SceneComponent.K2_GetComponentRotation` _camera) (`KismetMathLibrary.FindLookAtRotation` (`SceneComponent.K2_GetComponentLocation` _camera) (`SceneComponent.GetSocketLocation` (`self.Mesh`) "Hips")) (`GameplayStatics.GetWorldDeltaSeconds`) 3.0) false false)
  (if (`self.isDead`)
    (`SceneComponent.K2_SetWorldLocation` (`self.Camera`) (`self.CameraDeathPos`) false false)))

(event `self.ReceiveBeginPlay`
  (set `PlayerController.bShowMouseCursor` true (`GameplayStatics.GetPlayerController` 0))
  (set `self.CurrentHealth` (`self.MaxHealth`))
  (bind _returnvalue (`GameplayStatics.GetActorOfClass` "/Game/Blueprints/HUD/DiceCapture.DiceCapture_C"))
  (if (`KismetSystemLibrary.IsValid` _returnvalue)
    (add `/Game/Blueprints/HUD/DiceCapture.OnGoodDieResult` _returnvalue (delegate `OnGoodDie`))
    (`self.EquipWeapon` (`self.CurrentWeapon`) (stale `OnGoodDie` _output_get) :!label _label)))

(event `OnGoodDie`
  (params (DieResult :type Integer))
  (bind _output_get (set `self.Current Die Level` DieResult))
  (if (> (`self.Ammo`) 0)
    (`self.EquipWeapon` (`self.TempWeapon`) (`self.Current Die Level`))
    (else
      (goto _label))))

(event `Pickup Weapon`
  (params (WeaponPickup :type "/Game/Blueprints/Weapons/WeaponBase Object Reference"))
  (`self.EquipWeapon` WeaponPickup (`self.Current Die Level`)))

(event `/Game/Blueprints/Interface/CanDamage.OnDamaged`
  (params (Damage :type Integer) (Knockback :type "Vector Structure"))
  (if (not (`self.isInvincible`))
    (`self.LaunchCharacter` Knockback true true)
    (set `self.CurrentHealth` (- (`self.CurrentHealth`) Damage))
    (`|ExecutionSequence`
      (:`then_0`
        (if (< (`self.CurrentHealth`) 1)
          (`self.Death`)))
      (:`then_1`
        (set `self.isInvincible` true)
        (`KismetSystemLibrary.Delay` 2.0)
        (set `self.isInvincible` false)))))

(event `Death`
  (`PrimitiveComponent.SetSimulatePhysics` (`self.Mesh`) true)
  (`self.DisableInput` null)
  (set `self.isDead` true)
  (set `self.CameraDeathPos` (`SceneComponent.K2_GetComponentLocation` (`self.Camera`)))
  (`PlayerController.SetViewTargetWithBlend` (`GameplayStatics.GetPlayerController` 0) (`GameplayStatics.GetPlayerCharacter` 0) 1.0 "VTBlend_Cubic" 0.0 false)
  (set `CharacterMovementComponent.MaxWalkSpeed` 0.0 (`self.CharacterMovement`))
  (`KismetSystemLibrary.Delay` 1.0)
  (`PrimitiveComponent.SetCollisionEnabled` (`self.CapsuleComponent`) "NoCollision")
  (`KismetSystemLibrary.Delay` 4.0)
  (bind _returnvalue (`GameplayStatics.GetCurrentLevelName` true))
  (`GameplayStatics.OpenLevel` (`KismetStringLibrary.Conv_StringToName` _returnvalue)))

(event `InputAction|Shoot`
  (params (Key :type "Key Structure"))
  (:`Pressed`
    (`KismetSystemLibrary.Delay` 0.01 :!label _label)
    (if (`self.CanLeadingShoot`)
      (`self.Shoot`))
    (bind _returnvalue (`KismetSystemLibrary.K2_SetTimerDelegate` (delegate `Shoot`) (`self.FireRate`) true))
    (set `self.FireRateTimer` _returnvalue))
  (:`Released`
    (`KismetSystemLibrary.K2_ClearAndInvalidateTimerHandle` (`self.FireRateTimer`))
    (set `self.CanLeadingShoot` false)
    (`KismetSystemLibrary.RetriggerableDelay` (`self.FireRate`))
    (set `self.CanLeadingShoot` true)))

(event `StartShootTimer`
  (goto _label))

(event `Shoot`
  (bind _ammo (`self.Ammo`))
  (if (not (`self.isDead`))
    (switch `/Game/Blueprints/Weapons/WeaponModel` (`/Game/Blueprints/Weapons/WeaponBase.WeaponModel` (`self.CurrentWeapon`))
      (:`NewEnumerator0`
        (`|PlayMontage` (`self.Mesh`) "/Game/Characters/Player/Anim/AnimM_AxeAttack.AnimM_AxeAttack"
          (:`then`
            _)))
      (:`NewEnumerator1`
        _)
      (:`NewEnumerator2`
        _)
      (:`NewEnumerator3`
        _))
    (for _index (range (+ (`self.SpreadCount`) 1))
      (bind _returnvalue (`|SpawnActorFromClass` (`self.bullet type`) (`self.GetTransform`) "Undefined" "OverrideRootScale" null null))
      (bind _output_get (set `self.Bullet` _returnvalue))
      (if (`KismetSystemLibrary.IsValid` _output_get)
        (bind _returnvalue_2 (`KismetMathLibrary.GreaterGreater_VectorRotator` (`KismetMathLibrary.Conv_RotatorToVector` (`KismetMathLibrary.MakeRotator` 0.0 0.0 (+ (`self.RotateOffset`) (`self.PlayerZRot`)))) (`KismetMathLibrary.MakeRotator` 0.0 0.0 (* (/ (`self.SpreadWidth`) (`KismetMathLibrary.Conv_IntToDouble` (`self.SpreadCount`))) (- (`KismetMathLibrary.Conv_IntToDouble` _index) (* (`self.SpreadCount`) 0.5))))))
        (set `/Game/Blueprints/Bullets/BulletBase.Direction` _returnvalue_2 (`self.Bullet`))
        (`self.K2_SetActorLocation` (`self.Bullet`) (+ (* _returnvalue_2 (* (`self.Size`) 100.0)) (`self.K2_GetActorLocation`)) false false)
        (`self.SetActorScale3D` (`self.Bullet`) (* (`KismetMathLibrary.Vector_One`) (`self.Size`)))
        (set `/Game/Blueprints/Bullets/BulletBase.Speed` (`self.Speed`) (`self.Bullet`))
        (set `/Game/Blueprints/Bullets/BulletBase.Lifespan` (`self.Lifespan`) (`self.Bullet`))
        (set `/Game/Blueprints/Bullets/BulletBase.Knockback` (`self.knockback`) (`self.Bullet`))
        (if (> (`self.Ammo`) 0)
          (`/Engine/EditorBlueprintResources/StandardMacros.DecrementInt` _ammo
            (:`  `
              (`KismetSystemLibrary.PrintString` (`KismetStringLibrary.Conv_IntToString` _ammo))
              (if (== (`self.Ammo`) 0)
                (`self.EquipWeapon` (`self.CurrentWeapon`) (`self.Current Die Level`))))))))))

(event `InputAxis|MoveVertical`
  (params (AxisValue :type "Float (single-precision)"))
  (bind (_returnvalue_roll _returnvalue_pitch _returnvalue_yaw) (`KismetMathLibrary.BreakRotator` (`PlayerCameraManager.GetCameraRotation` (`GameplayStatics.GetPlayerCameraManager` 0))))
  ;[1 1 1] MoveInput
  (if (not (`self.isDead`))
    (set `self.MoveInput` (+ (* (`KismetMathLibrary.GetForwardVector` (`KismetMathLibrary.MakeRotator` 0.0 0.0 _returnvalue_yaw)) AxisValue) (`self.MoveInput`)))))

(event `InputAxis|MoveHorizontal`
  (params (AxisValue :type "Float (single-precision)"))
  (bind (_returnvalue_roll _returnvalue_pitch _returnvalue_yaw) (`KismetMathLibrary.BreakRotator` (`PlayerCameraManager.GetCameraRotation` (`GameplayStatics.GetPlayerCameraManager` 0))))
  ;[1 1 1] MoveInput
  (if (not (`self.isDead`))
    (set `self.MoveInput` (+ (* (`KismetMathLibrary.GetRightVector` (`KismetMathLibrary.MakeRotator` 0.0 0.0 _returnvalue_yaw)) AxisValue) (`self.MoveInput`)))))

(event `InputAxis|AimHorizontal`
  (params (AxisValue :type "Float (single-precision)"))
  (bind (_returnvalue_roll _returnvalue_pitch _returnvalue_yaw) (`KismetMathLibrary.BreakRotator` (`PlayerCameraManager.GetCameraRotation` (`GameplayStatics.GetPlayerCameraManager` 0))))
  ;[1 1 1] Aim
  (set `self.AimInput` (+ (* (`KismetMathLibrary.GetForwardVector` (`KismetMathLibrary.MakeRotator` 0.0 0.0 _returnvalue_yaw)) AxisValue) (`self.AimInput`))))

(event `InputAxis|AimVertical`
  (params (AxisValue :type "Float (single-precision)"))
  (bind (_returnvalue_roll _returnvalue_pitch _returnvalue_yaw) (`KismetMathLibrary.BreakRotator` (`PlayerCameraManager.GetCameraRotation` (`GameplayStatics.GetPlayerCameraManager` 0))))
  ;[1 1 1] Aim
  (set `self.AimInput` (+ (* (`KismetMathLibrary.GetRightVector` (`KismetMathLibrary.MakeRotator` 0.0 0.0 _returnvalue_yaw)) AxisValue) (`self.AimInput`))))

(event `InputAction|MouseClick`
  (params (Key :type "Key Structure"))
  ;[1 1 1] Mouse Aim Ovveride
  (:`Pressed`
    (bind _output_get (set `self.MouseOverride` true))
    (set `self.MousePressed` _output_get))
  (:`Released`
    (set `self.MousePressed` false)
    (`KismetSystemLibrary.RetriggerableDelay` 0.5)
    (if (not (`self.MousePressed`))
      (set `self.MouseOverride` false))))

(fn `EquipWeapon`
  (params (NewWeapon :type "/Game/Blueprints/Weapons/WeaponBase Object Reference") (Level :type Integer))
  (locals (Weapon :type "/Game/Blueprints/Weapons/WeaponBase Object Reference"))
  (bind _weapon (`local.Weapon`))
  (if (> (`/Game/Blueprints/Weapons/WeaponBase.Ammo` NewWeapon) 0)
    (bind _output_get (set `self.TempWeapon` NewWeapon))
    (bind _output_get_2 (set `local.Weapon` _output_get))
    (set `self.Ammo` (`/Game/Blueprints/Weapons/WeaponBase.Ammo` _output_get_2))
    (else
      (bind _output_get_3 (set `local.Weapon` NewWeapon))
      (set `self.CurrentWeapon` _output_get_3)))
  (`/Game/Blueprints/Weapons/WeaponBase.OnGoodRoll` _output_get_3 Level)
  (set `self.bullet type` (`/Game/Blueprints/Weapons/WeaponBase.Bullet Type` (`local.Weapon`)))
  (set `self.Size` (`/Game/Blueprints/Weapons/WeaponBase.Size` (`local.Weapon`)))
  (set `self.FireRate` (`/Game/Blueprints/Weapons/WeaponBase.FireRate` (`local.Weapon`)))
  (set `self.Speed` (`/Game/Blueprints/Weapons/WeaponBase.Speed` (`local.Weapon`)))
  (set `self.Damage` (`/Game/Blueprints/Weapons/WeaponBase.Damage` (`local.Weapon`)))
  (set `self.SpreadCount` (`/Game/Blueprints/Weapons/WeaponBase.SpreadCount` (`local.Weapon`)))
  (set `self.SpreadWidth` (`/Game/Blueprints/Weapons/WeaponBase.SpreadWidth` (`local.Weapon`)))
  (set `self.Lifespan` (`/Game/Blueprints/Weapons/WeaponBase.LifeSpan` (`local.Weapon`)))
  (set `self.knockback` (`/Game/Blueprints/Weapons/WeaponBase.Knockback` _weapon))
  (`SceneComponent.SetVisibility` (`self.Axe`) false false)
  (switch `/Game/Blueprints/Weapons/WeaponModel` (`/Game/Blueprints/Weapons/WeaponBase.WeaponModel` _weapon)
    (:`NewEnumerator0`
      (`SceneComponent.SetVisibility` (`self.Axe`) true false))
    (:`NewEnumerator1`
      _)
    (:`NewEnumerator2`
      _)
    (:`NewEnumerator3`
      _))
  (if (`KismetSystemLibrary.K2_IsTimerActiveHandle` (`self.FireRateTimer`))
    (`KismetSystemLibrary.K2_ClearAndInvalidateTimerHandle` (`self.FireRateTimer`))
    (`self.StartShootTimer`)))

(fn `PlayerRotate`
  (bind (_rotatehelper_roll _rotatehelper_pitch _rotatehelper_yaw) (`KismetMathLibrary.BreakRotator` (`self.RotateHelper`)))
  (bind (_returnvalue_roll _returnvalue_pitch _returnvalue_yaw) (`KismetMathLibrary.BreakRotator` (`KismetMathLibrary.MakeRotFromZ` (`self.AimInput`))))
  (bind (_returnvalue_roll_2 _returnvalue_pitch_2 _returnvalue_yaw_2) (`KismetMathLibrary.BreakRotator` (`KismetMathLibrary.MakeRotFromX` (`self.MoveInput`))))
  (if (> (`KismetMathLibrary.VSize` (`self.MoveInput`)) 0.01)
    (set `self.PlayerZRot` _returnvalue_yaw_2))
  (if (or (`self.MouseOverride`) (> (`KismetMathLibrary.VSize` (`self.AimInput`)) 0.01))
    (if (`self.MouseOverride`)
      (bind _yaw (`self.RotateTowardsMouse`))
      (set `self.RotateOffset` _yaw)
      (else
        (set `self.RotateOffset` (- _returnvalue_yaw (`self.PlayerZRot`)))))
    (else
      (set `self.RotateOffset` 0.0)))
  (`self.K2_SetActorRotation` (`self.RotateHelper`))
  (set `self.RotateHelper` (`KismetMathLibrary.RInterpTo` (`KismetMathLibrary.MakeRotator` 0.0 0.0 _rotatehelper_yaw) (`KismetMathLibrary.MakeRotator` 0.0 0.0 (`self.PlayerZRot`)) (`self.Delta Seconds`) 25.0)))

(fn `RotateTowardsMouse`
  (returns (Yaw :type "Float (double-precision)"))
  (locals (ReturnYaw :type "Float (double-precision)" :default 0.0))
  (bind (_worldlocation _worlddirection) (`PlayerController.DeprojectMousePositionToWorld` (`GameplayStatics.GetPlayerController` 0)))
  (bind _outhit (`KismetSystemLibrary.LineTraceSingle` _worldlocation (+ _worldlocation (* _worlddirection 100000.0)) "TraceTypeQuery1"))
  (if (`GameplayStatics.BreakHitResult` _outhit)
    (bind (_returnvalue_roll _returnvalue_pitch _returnvalue_yaw) (`KismetMathLibrary.BreakRotator` (`KismetMathLibrary.MakeRotFromX` (- (`KismetMathLibrary.SelectVector` (`self.K2_GetActorLocation` (`.HitActor` (`GameplayStatics.BreakHitResult` _outhit))) (`.Location` (`GameplayStatics.BreakHitResult` _outhit)) (`KismetSystemLibrary.DoesImplementInterface` (`.HitActor` (`GameplayStatics.BreakHitResult` _outhit)) "/Game/Blueprints/Interface/Enemy.Enemy_C")) (`self.K2_GetActorLocation`)))))
    (set `local.ReturnYaw` (- _returnvalue_yaw (`self.PlayerZRot`)))
    (else
      (set `local.ReturnYaw` 0.0)))
  (return (`local.ReturnYaw`)))

(fn `UserConstructionScript`)