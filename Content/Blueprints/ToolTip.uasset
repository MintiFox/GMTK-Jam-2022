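; One-shot trigger volume actor that shows or hides an on-screen tooltip when the Player enters its box.
; Each instance creates its own Tooltip widget and adds it to the viewport on BeginPlay.
; On overlap, the ShowTooltip flag selects either showing the message on that widget with duration, font size and slowdown, or hiding the first Tooltip widget found in the viewport.
; Both paths then destroy the actor.
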(event `self.ReceiveBeginPlay`
  (bind _returnvalue (`|CreateWidget` "/Game/Blueprints/HUD/Tooltip.Tooltip_C"))
  (bind _output_get (set `self.HUD_Tooltip` _returnvalue))
  (`UserWidget.AddToViewport` _output_get 0))

(event `self.Box.OnComponentBeginOverlap`
  (params (OverlappedComponent :type "PrimitiveComponent Object Reference") (OtherActor :type "Actor Object Reference") (OtherComp :type "PrimitiveComponent Object Reference") (OtherBodyIndex :type Integer) (bFromSweep :type Boolean) (SweepResult :type "HitResult Structure (by ref)"))
  (cast `/Game/Blueprints/Player/Player` OtherActor)
  (if (`self.showTooltip`)
    (`/Game/Blueprints/HUD/Tooltip.ShowTooltip` (`self.HUD_Tooltip`) (`self.Duration`) (`self.Message`) (`self.fontSize`) (`self.slowdown?`))
    (`self.K2_DestroyActor`)
    (else
      (bind _foundwidgets (`WidgetBlueprintLibrary.GetAllWidgetsOfClass` "/Game/Blueprints/HUD/Tooltip.Tooltip_C"))
      (bind _astooltip (cast `/Game/Blueprints/HUD/Tooltip` (`|GetArrayItem` _foundwidgets)))
      (`/Game/Blueprints/HUD/Tooltip.HideTooltip` _astooltip)
      (`self.K2_DestroyActor`))))

(fn `UserConstructionScript`)